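; BP_Interactable is an interactable actor that currently gives the player a weapon as soon as play begins.
; On BeginPlay, a DoOnce spawns the Item class at the player character's transform, with the player as owner and instigator, then calls OnEquipped on it.
; Both Interact handlers are empty stubs.
; The pickup message, sheath sound and Quest hiding are disconnected and never run.
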(event `self.ReceiveBeginPlay`
  (bind _returnvalue (`GameplayStatics.GetPlayerCharacter` 0))
  ;[1 0 0] Spawns Weapon on Player
  (`/Engine/EditorBlueprintResources/StandardMacros.DoOnce` false
    (:`Completed`
      (bind _returnvalue_2 (`|SpawnActorFromClass` (`self.Item`) (`self.GetTransform` _returnvalue) "Undefined" "MultiplyWithRoot" _returnvalue _returnvalue))
      (`/Game/03_GameplayAssets/01_Weapon/BP_BaseEquippable.OnEquipped` _returnvalue_2))))

(event `Interact_1_1`
  (params (Caller :type "Actor Object Reference"))
  ;[1 0 0] Spawns Weapon on Player
)

(fn `Interact`
  (params (Caller :type "Actor Object Reference"))
  (returns (ObjectiveID :type String))
  (return ""))

(fn `UserConstructionScript`)