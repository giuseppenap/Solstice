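; BP_BaseWeapon is the base weapon: an equippable item that deals point damage on hit.
; On BeginPlay it registers as its owning third-person character's MainWeapon.
; Equipping attaches it to the hand socket, registers it with BP_CombatComponent, sends its combat type to the AnimInstance and configures its collision component to ignore the owner.
; Collision hits apply Damage along the owner's forward vector; OnUnequipped sets IsEquipped to true if already equipped.
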(event `self.ReceiveBeginPlay`
  (`parent.ReceiveBeginPlay`)
  (bind _asbp_third_person_character (cast `/Game/04_Characters/01_Player/BP_ThirdPersonCharacter` (`self.GetOwner`)))
  (set `/Game/04_Characters/01_Player/BP_ThirdPersonCharacter.MainWeapon` self _asbp_third_person_character))

(event `self.BP_CollisionComponent.OnHit`
  (params (HitResult :type "HitResult Structure"))
  (`GameplayStatics.ApplyPointDamage` (`.HitActor` (`GameplayStatics.BreakHitResult` HitResult)) (`self.Damage`) (`self.GetActorForwardVector` (`self.GetOwner`)) HitResult (`self.GetInstigatorController`) self))

(fn `OnEquipped`
  (`self.SetIsEquipped` true)
  (bind _output_get (set `self.CombatCombatComponent` (`self.GetComponentByClass` (`self.GetOwner`) "/Game/03_GameplayAssets/03_Combat/BP_CombatComponent.BP_CombatComponent_C")))
  (`/Engine/EditorBlueprintResources/StandardMacros.IsValid` _output_get
    (:`Is Valid`
      (`self.AttachActor` (`self.HandSocketName`))
      (`/Game/03_GameplayAssets/03_Combat/BP_CombatComponent.SetMainWeapon` (`self.CombatCombatComponent`) self)
      (message `/Game/03_GameplayAssets/04_Interfaces/BPI_AnimInstance.UpdateCombatType` (`SkeletalMeshComponent.GetAnimInstance` (`Character.Mesh` (cast `Character` (`self.GetOwner`) :!pure true))) (`self.Combat Type`))
      (`/Game/03_GameplayAssets/03_Combat/BP_CollisionComponent.SetCollisionMesh` (`self.BP_CollisionComponent`) (`self.GetItemMesh`))
      (`/Game/03_GameplayAssets/03_Combat/BP_CollisionComponent.AddActorsToIgnore` (`self.BP_CollisionComponent`) (`self.GetOwner`)))))

(fn `OnUnequipped`
  (`parent.OnUnequipped`)
  (if (`self.IsEquipped?`)
    (`self.SetIsEquipped` true)))

(fn `UserConstructionScript`
  (`parent.UserConstructionScript`))