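; BP_StateManagerComponent is a combat component that tracks a single current state for its owner.
; SetState ignores unchanged values; otherwise it fires the state-end call for the old state, stores the new one, then fires the state-begin call.
; ResetState returns to a default enum value, and helper functions return the current state or check it against a list of states.
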(fn `GetCurrentState`
  (returns (CurrentState :type "/Game/04_Characters/01_Player/Enums/E_CharacterState Enum"))
  (return (`self.CurrentState`)))

(fn `IsCurrentStateEqualToAny?`
  (params (StatesToCheck :type "Array of /Game/04_Characters/01_Player/Enums/E_CharacterState Enum"))
  (returns (ReturnValue :type Boolean))
  (return (`KismetArrayLibrary.Array_Contains` StatesToCheck (`self.CurrentState`))))

(fn `ResetState`
  (`self.SetState` "NewEnumerator0"))

(fn `SetState`
  (params (`New State` :type "/Game/04_Characters/01_Player/Enums/E_CharacterState Enum" :default "NewEnumerator0"))
  (bind _new_state (`local.New State`))
  (if (`|EnumInequality` `New State` (`self.CurrentState`))
    (`self.OnStateEnd` (`self.CurrentState`))
    (set `self.CurrentState` _new_state)
    (`self.OnStateBegin` _new_state)))