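; Combat collision component that detects hits along a mesh, swept between two sockets while collision is enabled.
; Each tick it runs a multi sphere trace for objects between the start and end sockets of the assigned mesh, skipping ignored actors.
; Each actor is reported through OnHit only once per activation, because enabling collision clears the already-hit list.
; Functions expose the ignore list, last hit and hit actors.
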(event `self.ReceiveTick`
  (params (DeltaSeconds :type "Float (single-precision)"))
  (if (`self.bIsCollisionEnabled?`)
    (`self.CollistionTrace`)))

(event `SetCollisionMesh`
  (params (MeshComponent :type "PrimitiveComponent Object Reference"))
  ;[1 0 0] Set Collision Mesh Component
  (set `self.CollisionMeshComponent` MeshComponent))

(event `CollistionTrace`
  ;[1 0 0] Collision Trace
  (bind _outhits (`KismetSystemLibrary.SphereTraceMultiForObjects` (`SceneComponent.GetSocketLocation` (`self.CollisionMeshComponent`) (`self.StartSocketName`)) (`SceneComponent.GetSocketLocation` (`self.CollisionMeshComponent`) (`self.EndSocketName`)) (`self.Trace Radius`) (`self.CollisionObjectTypes`) false (`self.Actors to Ignore`) (`self.Draw Debug Type`)))
  (for _array_element _outhits
    (bind _output_get (set `self.LastHit` _array_element))
    (bind (_bblockinghit _binitialoverlap _time _distance _location _impactpoint _normal _impactnormal _physmat _hitactor) (`GameplayStatics.BreakHitResult` _output_get))
    (if (not (`KismetArrayLibrary.Array_Contains` (`self.AlreadyHitActors`) _hitactor))
      (bind _output_get_2 (set `self.Hit Actor` _hitactor))
      (`KismetArrayLibrary.Array_Add` (`self.AlreadyHitActors`) _output_get_2)
      (`self.OnHit` (`self.LastHit`)))))

(event `EnableCollision`
  ;[1 0 0] Enable Collision
  (`self.ClearHitActors`)
  (set `self.bIsCollisionEnabled?` true))

(event `DisableCollision`
  ;[1 0 0] Disable Collision
  (set `self.bIsCollisionEnabled?` false))

(event `ClearHitActors`
  ;[1 0 0] Clear Hit actors
  (`KismetArrayLibrary.Array_Clear` (`self.AlreadyHitActors`)))

(fn `AddActorsToIgnore`
  (params (`In Actor` :type "Actor Object Reference (by ref)"))
  (`KismetArrayLibrary.Array_AddUnique` (`self.Actors to Ignore`) `In Actor`))

(fn `GetActorsToIgnore`
  (returns (`Return Value` :type "Array of Actor Object Reference"))
  (return (`self.Actors to Ignore`)))

(fn `GetAlreadyHitActors`
  (returns (ReturnValue :type "Array of Actor Object Reference"))
  (return (`self.AlreadyHitActors`)))

(fn `GetCollisionMeshComponent`
  (returns (`Return Value` :type "PrimitiveComponent Object Reference"))
  (return (`self.CollisionMeshComponent`)))

(fn `GetLastHit`
  (returns (`Return Value` :type "HitResult Structure"))
  (return (`self.LastHit`)))

(fn `IsCollisionEnabled?`
  (returns (`Return Value` :type Boolean))
  (return (`self.bIsCollisionEnabled?`)))

(fn `RemoveActorToIgnore`
  (params (`Actor To Remove` :type "Actor Object Reference (by ref)"))
  (`KismetArrayLibrary.Array_RemoveItem` (`self.Actors to Ignore`) `Actor To Remove`))